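; BP_Enemy is an enemy actor that damages the player on contact and can be destroyed by projectiles.
; When its Box overlaps BP_Player, it lowers the player's health, raises the score and plays a camera shake at the player's camera before destroying itself.
; When a BP_Projectile overlaps it, both actors are destroyed with no score change.
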(event OnComponentBeginOverlap(Box)
  (params (OverlappedComponent :type Primitive%20Component%20Object%20Reference) (OtherActor :type Actor%20Object%20Reference) (OtherComp :type Primitive%20Component%20Object%20Reference) (OtherBodyIndex :type Integer) (bFromSweep :type Boolean) (SweepResult :type Hit%20Result%20Structure%20%28by%20ref%29))
  (bind _asbp_player (Utilities|Casting|CastToBP_Player OtherActor)
    (:then
      (Default|ChangeHealth _asbp_player (- (Variables|/Game/InfiniteMatrix/Blueprints/BP_Player.BP_Player_C|GetHealth _asbp_player) 0.34))
      (Default|ChangeScore _asbp_player (+ (Variables|/Game/InfiniteMatrix/Blueprints/BP_Player.BP_Player_C|GetScore _asbp_player) 1))
      (Camera|PlayWorldCameraShake "/Game/InfiniteMatrix/Blueprints/BP_CameraShake.BP_CameraShake_C" (Transformation|GetWorldLocation (Variables|/Game/InfiniteMatrix/Blueprints/BP_Player.BP_Player_C|GetCamera _asbp_player)) 0.0 1e+04))
    (:CastFailed
      (bind _asbp_projectile (Utilities|Casting|CastToBP_Projectile OtherActor))
      (Actor|DestroyActor _asbp_projectile)))
  (Actor|DestroyActor))

(event EventBeginPlay)

(event Collision|EventActorBeginOverlap
  (params (OtherActor :type Actor%20Object%20Reference)))

(event EventTick
  (params (DeltaSeconds :type Float%20%28single-precision%29)))

(fn ConstructionScript)