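; BP_Projectile is a projectile actor in the InfiniteMatrix game that flies in a straight line along the world X axis.
; Each Tick moves the root component forward by Speed times delta time, keeping Y and Z unchanged, without a projectile movement component.
; When its collision mesh begins overlapping a BP_Tunnel, it destroys itself; other overlaps are ignored.
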(event OnComponentBeginOverlap(CollisionMesh)
  (params (OverlappedComponent :type Primitive%20Component%20Object%20Reference) (OtherActor :type Actor%20Object%20Reference) (OtherComp :type Primitive%20Component%20Object%20Reference) (OtherBodyIndex :type Integer) (bFromSweep :type Boolean) (SweepResult :type Hit%20Result%20Structure%20%28by%20ref%29))
  (Utilities|Casting|CastToBP_Tunnel OtherActor)
  (Actor|DestroyActor))

(event EventBeginPlay)

(event Collision|EventActorBeginOverlap
  (params (OtherActor :type Actor%20Object%20Reference)))

(event EventTick
  (params (DeltaSeconds :type Float%20%28single-precision%29))
  (bind _returnvalue (Transformation|GetActorLocation))
  (bind (_x _y _z) (Class|KismetMathLibrary|BreakVector3f _returnvalue))
  (Transformation|SetWorldLocation (Variables|Default|GetDefaultSceneRoot) (Math|Vector|MakeVector (+ (* (Variables|Default|GetSpeed) DeltaSeconds) (.X (Class|KismetMathLibrary|BreakVector3f (Transformation|GetWorldLocation (Variables|Default|GetDefaultSceneRoot))))) _y _z) false false))

(fn ConstructionScript)